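; Spider actor for level 2, a timed tapping challenge where each click nudges it along the Y axis while time remains.
; BeginPlay briefly blocks input, then starts game music and adds a Tapping_spot widget.
; A one-second retriggerable-delay loop runs Countdown, creating a new time widget each tick.
; At zero it shows Defeat unless the game instance's Level2Victory flag is set, in which case it clears that flag.
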(event Custom|moving%20Front
  (bind _output_get (Variables|Default|SetSetting%20Distance (+ (Transformation|GetActorLocation) "0.000000,15.000000,0.000000")))
  (Transformation|SetActorLocation self _output_get false false))

(event Custom|Clicked
  (if (> (Variables|Default|GetTime) 0)
    (CallFunction|MovingFront)))

(event Custom|Counting%20TIme
  (CallFunction|Countdown))

(event EventBeginPlay
  (Input|DisableInput (Game|GetPlayerController 0))
  (Utilities|FlowControl|Delay 4.0)
  (Input|EnableInput (Game|GetPlayerController 0))
  (Utilities|FlowControl|Sequence
    (:then_0
      (bind _asmultiplayer_game_instance (Utilities|Casting|CastToMultiplayer_game_instance (Game|GetGameInstance)))
      (if (not (Variables|/Game/For_multiplayer/Multiplayer_game_instance.Multiplayer_game_instance_C|GetLevel_2_victory _asmultiplayer_game_instance))
        (CallFunction|CountingTIme :!label _label)
        (Utilities|FlowControl|RetriggerableDelay 1.0)
        (goto _label)))
    (:then_1
      ;[1 1 1] Playing In game music
      (if (> (Variables|Default|GetTime) 1)
        _
        (else
          _))
      (bind _asmultiplayer_game_instance_2 (Utilities|Casting|CastToMultiplayer_game_instance (Game|GetGameInstance)))
      (if (Variables|/Game/For_multiplayer/Multiplayer_game_instance.Multiplayer_game_instance_C|GetPlaying%20music _asmultiplayer_game_instance_2)
        (bind _asmultiplayer_game_instance_3 (Utilities|Casting|CastToMultiplayer_game_instance (Game|GetGameInstance)))
        (Default|StartPlayingIngameMusic _asmultiplayer_game_instance_3)))
    (:then_2
      (bind _returnvalue (UserInterface|CreateWidget "/Game/Widgets/Tapping_spot.Tapping_spot_C"))
      (UserInterface|Viewport|AddtoViewport _returnvalue 0))))

(event EventActorBeginOverlap
  (params (OtherActor :type Actor%20Object%20Reference)))

(event Input|ActionEvents|InputActioncountingNumberofclicks
  (params (Key :type Key%20Structure :default "AnyKey")))

(fn ConstructionScript)

(fn Countdown
  (if (> (Variables|Default|GetTime) 0)
    (bind _result (Math|Integer|DecrementInt (Variables|Default|GetTime))
      (:%20%20
        (bind _output_get (Variables|Default|SetTime _result))
        (if (== (Variables|Default|GetTime) 0)
          (bind _asmultiplayer_game_instance (Utilities|Casting|CastToMultiplayer_game_instance (Game|GetGameInstance)))
          (if (Variables|/Game/For_multiplayer/Multiplayer_game_instance.Multiplayer_game_instance_C|GetLevel_2_victory _asmultiplayer_game_instance)
            (bind _asmultiplayer_game_instance_2 (Utilities|Casting|CastToMultiplayer_game_instance (Game|GetGameInstance)))
            (Variables|/Game/For_multiplayer/Multiplayer_game_instance.Multiplayer_game_instance_C|SetLevel_2_victory _asmultiplayer_game_instance_2 false)
            (else
              (bind _returnvalue (UserInterface|CreateWidget "/Game/Widgets/Defeat.Defeat_C" (Game|GetPlayerController 0)))
              (UserInterface|Viewport|AddtoViewport _returnvalue 0)))
          (else
            (bind _returnvalue_2 (UserInterface|CreateWidget "/Game/Widgets/Time_level_2.Time_level_2_C"))
            (Variables|/Game/Widgets/Time_level_2.Time_level_2_C|SetGame_time _returnvalue_2 (Utilities|String|ToString(Integer) _output_get))
            (UserInterface|Viewport|AddtoViewport _returnvalue_2 0)))))))