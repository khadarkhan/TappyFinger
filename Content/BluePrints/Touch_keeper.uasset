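; Touch_keeper runs a timed click-counting round, adding to the player state's score on each press while time remains.
; After a short input-locked delay, BeginPlay starts in-game music and a one-second countdown loop that adds a new Time widget each tick.
; At zero it writes the score to the leaderboard and game instance, then shows Victory, level 2 unlock or Defeat.
; The Save_score object is created fresh and never written to a slot.
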(event Custom|Counting%20Time
  ;[1 1 1] Time count down event
  (if (> (Variables|Default|GetTime) 0)
    (CallFunction|Countdown)))

(event Custom|Client%20counting%20number%20of%20clicks
  ;[1 1 1] counts the number of clicks
  (CallFunction|NumberOfClicks))

(event EventBeginPlay
  ;[1 1 1] calls Time count down event
  (Input|DisableInput (Game|GetPlayerController 0))
  (Utilities|FlowControl|Delay 4.0)
  (Input|EnableInput (Game|GetPlayerController 0))
  (Utilities|FlowControl|Sequence
    (:then_0
      (CallFunction|CountingTime :!label _label)
      (Utilities|FlowControl|RetriggerableDelay 1.0)
      (goto _label))
    (:then_1
      ;[1 1 1] Playing In game music
      (if (> (Variables|Default|GetTime) 1)
        _
        (else
          _))
      (bind _asmultiplayer_game_instance (Utilities|Casting|CastToMultiplayer_game_instance (Game|GetGameInstance)))
      (if (Variables|/Game/For_multiplayer/Multiplayer_game_instance.Multiplayer_game_instance_C|GetPlaying%20music _asmultiplayer_game_instance)
        (bind _asmultiplayer_game_instance_2 (Utilities|Casting|CastToMultiplayer_game_instance (Game|GetGameInstance)))
        (Default|StartPlayingIngameMusic _asmultiplayer_game_instance_2)))))

(event Input|ActionEvents|InputActioncountingNumberofclicks
  (params (Key :type Key%20Structure :default "AnyKey"))
  ;[1 1 1] calls the number of clicks event
  (:Pressed
    (if (> (Variables|Default|GetTime) 0)
      (CallFunction|ClientCountingNumberOfClicks)
      (bind _asmultiplayer_game_instance (Utilities|Casting|CastToMultiplayer_game_instance (Game|GetGameInstance)))
      (if (Variables|/Game/For_multiplayer/Multiplayer_game_instance.Multiplayer_game_instance_C|GetPlaying%20music _asmultiplayer_game_instance)
        (Audio|SpawnSound2D "/Game/Sound_effects/ButtonPush_2.ButtonPush_2")))))

(fn ConstructionScript)

(fn NumberOfClicks
  (bind _asmultiplayer_my_player_state (Utilities|Casting|CastToMultiplayerMyPlayerState (Variables|GetPlayerState)))
  (Default|IncrementScore _asmultiplayer_my_player_state))

(fn Countdown
  ;[1 1 1] Calculating Time, Displaying Time, displaying game Over widget and Giving score to Leadership board
  (if (> (Variables|Default|GetTime) 0)
    (bind _result (Math|Integer|DecrementInt (Variables|Default|GetTime))
      (:%20%20
        (bind _output_get (Variables|Default|SetTime _result))
        (if (== (Variables|Default|GetTime) 0)
          (bind _asmultiplayer_my_player_state (Utilities|Casting|CastToMultiplayerMyPlayerState (Variables|GetPlayerState)))
          (Class|LeaderboardBlueprintLibrary|WriteLeaderboardInteger (Game|GetPlayerController 0) "High Score" (Variables|/Game/For_multiplayer/MultiplayerMyPlayerState.MultiplayerMyPlayerState_C|GetPlayerScore _asmultiplayer_my_player_state))
          (bind _asmultiplayer_game_instance (Utilities|Casting|CastToMultiplayer_game_instance (Game|GetGameInstance)))
          (Default|GettingPlayerScore _asmultiplayer_game_instance (Variables|/Game/For_multiplayer/MultiplayerMyPlayerState.MultiplayerMyPlayerState_C|GetPlayerScore _asmultiplayer_my_player_state))
          (if (>= (Variables|/Game/For_multiplayer/MultiplayerMyPlayerState.MultiplayerMyPlayerState_C|GetPlayerScore _asmultiplayer_my_player_state) 100)
            (bind _returnvalue (SaveGame|CreateSaveGameObject "/Game/BluePrints/Save_score.Save_score_C"))
            (bind _assave_score (Utilities|Casting|CastToSave_score _returnvalue))
            (Variables|/Game/BluePrints/Save_score.Save_score_C|SetScore _assave_score (Variables|/Game/For_multiplayer/MultiplayerMyPlayerState.MultiplayerMyPlayerState_C|GetPlayerScore _asmultiplayer_my_player_state))
            (if (Variables|/Game/BluePrints/Save_score.Save_score_C|GetScore%20stored _assave_score)
              (bind _returnvalue_2 (UserInterface|CreateWidget "/Game/Widgets/Victory.Victory_C" (Game|GetPlayerController 0)))
              (UserInterface|Viewport|AddtoViewport _returnvalue_2 0)
              (else
                (bind _returnvalue_3 (UserInterface|CreateWidget "/Game/Widgets/Unlocked_level_2.Unlocked_level_2_C"))
                (UserInterface|Viewport|AddtoViewport _returnvalue_3 0)
                (Variables|/Game/BluePrints/Save_score.Save_score_C|SetScore%20stored _assave_score true)))
            (else
              (bind _returnvalue_4 (UserInterface|CreateWidget "/Game/Widgets/Defeat.Defeat_C" (Game|GetPlayerController 0)))
              (UserInterface|Viewport|AddtoViewport _returnvalue_4 0)))
          (else
            (bind _returnvalue_5 (UserInterface|CreateWidget "/Game/Widgets/Time.Time_C"))
            (Variables|/Game/Widgets/Time.Time_C|SetGame_time _returnvalue_5 (Utilities|String|ToString(Integer) _output_get))
            (UserInterface|Viewport|AddtoViewport _returnvalue_5 0)))))))

(fn ShowWidget
  (bind _returnvalue (UserInterface|CreateWidget "/Game/Widgets/Defeat.Defeat_C"))
  (UserInterface|Viewport|AddtoViewport _returnvalue 0))